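; BP_LobbyGM is the lobby game mode that tracks players as they join.
; On PostLogin it sets UserCount on BP_LobbyGS from the PlayerArray length.
; With authority, it calls OnRepUserCount directly on the game state and adds the new controller to AllPlayerControllers.
; BeginPlay, Tick and the construction script are empty, and no logout handling appears.
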(event EventBeginPlay)

(event EventTick
  (params (DeltaSeconds :type Float%20%28single-precision%29)))

(event EventPostLogin
  (params (NewPlayer :type Player%20Controller%20Object%20Reference))
  (bind _asbp_lobby_gs (Utilities|Casting|CastToBP_LobbyGS (Game|GetGameState)))
  (Utilities|IsValid _asbp_lobby_gs
    (:Is%20Valid
      (Variables|/Game/Blueprints/Lobby/BP_LobbyGS.BP_LobbyGS_C|SetUserCount _asbp_lobby_gs (Utilities|Array|Length (Variables|/Script/Engine.GameStateBase|GetPlayerArray _asbp_lobby_gs)))
      (if (Ability|HasAuthority)
        (Default|OnRepUserCount _asbp_lobby_gs)
        (Utilities|Array|Add (Variables|Default|GetAllPlayerControllers) NewPlayer)))))

(fn ConstructionScript)