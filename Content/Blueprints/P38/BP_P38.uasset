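; BP_P38 is a player-controlled P-38 plane pawn that flies forward constantly and fires rockets.
; Tick feeds forward movement input and spins the left and right propellers through the shared RotatePropellar function, scaled by delta time and RotateSpeed.
; Pitch and Roll axes rotate the plane locally at PlaneRotateSpeed, also scaled by delta time.
; Pressing Fire spawns a BP_Rocket at the Arrow component's world transform.
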(event EventBeginPlay)

(event Collision|EventActorBeginOverlap
  (params (OtherActor :type Actor%20Object%20Reference)))

(event EventTick
  (params (DeltaSeconds :type Float%20%28single-precision%29))
  (Pawn|Input|AddMovementInput (Transformation|GetActorForwardVector) 1.0 false)
  (CallFunction|RotatePropellar (Variables|Default|GetPropellar_L))
  (CallFunction|RotatePropellar (Variables|Default|GetPropellar_R)))

(event Input|ActionEvents|InputActionFire
  (params (Key :type Key%20Structure))
  (:Pressed
    (Game|SpawnActorfromClass "/Game/Blueprints/P38/BP_Rocket.BP_Rocket_C" (Transformation|GetWorldTransform (Variables|Default|GetArrow)) "Undefined" 0 0)))

(event Input|AxisEvents|InputAxisPitch
  (params (AxisValue :type Float%20%28single-precision%29))
  (Transformation|AddActorLocalRotation (Math|Rotator|MakeRotator 0.0 (* AxisValue (Utilities|Time|GetWorldDeltaSeconds) (Variables|Default|GetPlaneRotateSpeed)) 0.0) false false))

(event Input|AxisEvents|InputAxisRoll
  (params (AxisValue :type Float%20%28single-precision%29))
  (Transformation|AddActorLocalRotation (Math|Rotator|MakeRotator (* AxisValue (Utilities|Time|GetWorldDeltaSeconds) (Variables|Default|GetPlaneRotateSpeed)) 0.0 0.0) false false))

(fn ConstructionScript)

(fn RotatePropellar
  (params (Propellar :type Scene%20Component%20Object%20Reference))
  (Transformation|AddLocalRotation Propellar (Math|Rotator|MakeRotator (* (Utilities|Time|GetWorldDeltaSeconds) (Variables|Default|GetRotateSpeed)) 0.0 0.0) false false))