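; BP_PC is a replicated player controller that gives each player a random character pawn from three classes.
; On BeginPlay the local controller picks a class, with RandomInteger(4) % 3 favoring the first, and passes it to ServerSetPawn.
; That event stores the class and calls RestartPlayer on BP_GM.
; GetPlayerPawnClass exposes the stored choice.
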(event Custom|DeterminePawnClass
  (if (Pawn|IsLocalController)
    (switch int (Math|Integer|%(Integer) (Math|Random|RandomInteger 4) 3)
      (:Default
        (CallFunction|ServerSetPawn (Variables|Default|GetPawnToUseA) :!label _label))
      (:0
        (goto _label))
      (:1
        (CallFunction|ServerSetPawn (Variables|Default|GetPawnToUseB)))
      (:2
        (CallFunction|ServerSetPawn (Variables|Default|GetPawnToUseC))))))

(event Custom|ServerSetPawn
  (params (InPawnClass :type Pawn%20Class%20Reference))
  (Variables|Default|SetMyPawnClass InPawnClass)
  (bind _asbp_gm (Utilities|Casting|CastToBP_GM (Game|GetGameMode)))
  (Class|GameModeBase|RestartPlayer _asbp_gm self))

(event EventBeginPlay
  (CallFunction|DeterminePawnClass)
  (if (Pawn|IsLocalController)
    (Development|PrintString (Utilities|GetDisplayName self))))

(event EventTick
  (params (DeltaSeconds :type Float%20%28single-precision%29)))

(fn ConstructionScript
  (Variables|Default|SetPawnToUseA "/Game/Blueprints/BP_MyCharacter.BP_MyCharacter_C")
  (Variables|Default|SetPawnToUseB "/Game/Blueprints/BP_MyCharacter1.BP_MyCharacter1_C")
  (Variables|Default|SetPawnToUseC "/Game/Blueprints/BP_MyCharacter2.BP_MyCharacter2_C")
  (Networking|SetReplicates true))

(fn GetPlayerPawnClass
  (return (Variables|Default|GetMyPawnClass)))